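; General game-state Blueprint that tracks playable and non-playable characters and manages an RPG tile mesh.
; On BeginPlay it sorts every TopDownCharacter into two arrays by actor tag, defaulting the tag to "Playable" if unset.
; MakeMeshRPG spawns a Casilla tile below the controlled pawn as its own parent and stores it as ActualMother.
; DestroyMeshRPG tells that root tile to destroy the whole mesh.
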(event EventBeginPlay
  (CallFunction|StartandAssingValues))

(fn ConstructionScript)

(fn StartandAssingValues
  ;[1 0.1264 0.697] Secure Condition
  (if (Utilities|Name|Equal(Name) (Variables|Default|GetPlayablePlayerTag) "None")
    (Variables|Default|SetPlayablePlayerTag "Playable"))
  (bind _outactors (Actor|GetAllActorsOfClass "/Game/TopDownBP/Blueprints/TopDownCharacter.TopDownCharacter_C"))
  (for _array_element _outactors
    ;[0 0.9243 1] BodyLoop
    (bind _output_get (LocalVariables|SetActualActor _array_element))
    (if (Actor|ActorHasTag _output_get (Variables|Default|GetPlayablePlayerTag))
      (Utilities|Array|Add (Variables|Default|GetPlayableActors) (LocalVariables|GetActualActor))
      (else
        (Utilities|Array|Add (Variables|Default|GetNoPlayableActors) (LocalVariables|GetActualActor))))))

(fn MakeMeshRPG
  (bind _returnvalue (Game|GetPlayerController 0))
  (bind _returnvalue_2 (Pawn|GetControlledPawn _returnvalue))
  (bind _returnvalue_3 (Transformation|GetActorTransform _returnvalue_2))
  (bind _returnvalue_4 (Game|SpawnActorfromClass "/Game/BluePrints/Casilla.Casilla_C" (Math|Transform|MakeTransform (Math|Vector|MakeVector (.x (.location _returnvalue_3)) (.y (.location _returnvalue_3)) (+ (.z (.location _returnvalue_3)) -155.0)) "0, 0, 0" "1,1,1") "Undefined" 0 0))
  (Variables|/Game/BluePrints/Casilla.Casilla_C|SetParentReference _returnvalue_4 _returnvalue_4)
  (Variables|Default|SetActualMother _returnvalue_4))

(fn DestroyMeshRPG
  (Default|DestroyAllMesh (Variables|Default|GetActualMother)))