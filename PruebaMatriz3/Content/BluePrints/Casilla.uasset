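; Casilla is a grid tile actor that flood-fills an area with copies of itself at runtime.
; After a short delay on BeginPlay, it box-traces its four neighboring positions, rejecting empty spots and hits tagged End or CubeMesh.
; Valid spots spawn a new Casilla attached to the shared ParentReference, which repeats the propagation recursively.
; Helper functions destroy attached actors with the tile and recolor it through a dynamic material.
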(event EventBeginPlay
  (Utilities|FlowControl|Delay 0.15)
  (CallFunction|PropageFourDirection))

(event EventTick
  (params (DeltaSeconds :type Float%20%28single-precision%29)))

(fn ConstructionScript)

(fn CheckColliders
  (params (Position :type Vector) (BoxSize :type Vector))
  (bind _outhits (Class|KismetSystemLibrary|BoxTraceMultiforObjects Position Position (* BoxSize 0.99) "0, 0, 0" (Variables|Default|GetLocalObjectTypeCompare) false 0 "None" true))
  ;[1 0.5625 0.5625] LoopBodyColliders
  (for _array_element _outhits
    (Utilities|FlowControl|Sequence
      (:then_0
        (LocalVariables|SetColliderLocalCount (+ (LocalVariables|GetColliderLocalCount) 1)))
      (:then_1
        ;;[1 0.2396 0.2396] LoopTags
        (for _array_element_2 (Variables|/Script/Engine.Actor|GetTags (.HitActor (Collision|BreakHitResult _array_element)))
          (if (or (Utilities|Enum|Equal(Enum) (Utilities|String|ToString(Name) _array_element_2) "End") (Utilities|Enum|Equal(Enum) (Utilities|String|ToString(Name) _array_element_2) "CubeMesh"))
            (LocalVariables|SetisWall true)
            (return false)
            (else
              (LocalVariables|SetisWall false)))))))
  (if (== (LocalVariables|GetColliderLocalCount) 0)
    (return false)
    (else
      (return true))))

(fn PropageFourDirection
  (bind _returnvalue (Transformation|GetActorLocation))
  (bind _boxsize (Variables|Default|GetBoxSize))
  (Utilities|FlowControl|Sequence
    (:then_0
      (LocalVariables|SetTranformationPropage (Math|Transform|MakeTransform (+ (* (Class|KismetMathLibrary|VectorForward) _boxsize) _returnvalue))))
    (:then_1
      (LocalVariables|SetTranformationPropage (Math|Transform|MakeTransform (+ (* (Class|KismetMathLibrary|VectorBackward) _boxsize) _returnvalue))))
    (:then_2
      (LocalVariables|SetTranformationPropage (Math|Transform|MakeTransform (+ (* (Class|KismetMathLibrary|VectorRight) _boxsize) _returnvalue))))
    (:then_3
      (LocalVariables|SetTranformationPropage (Math|Transform|MakeTransform (+ (* (Class|KismetMathLibrary|VectorLeft) _boxsize) _returnvalue)))))
  (bind _propage (CallFunction|CheckColliders (.location (LocalVariables|GetTranformationPropage)) (.BoxExtent (Collision|GetActorBounds false false))))
  (if _propage
    ;[0.1816 0.4214 1] Recursividad
    (bind _returnvalue_2 (Game|SpawnActorfromClass "Casilla_C" (LocalVariables|GetTranformationPropage) "Undefined" 0 0))
    (Variables|Casilla_C|SetParentReference _returnvalue_2 (Variables|Default|GetParentReference))
    (Transformation|AttachActorToActor _returnvalue_2 (Variables|Default|GetParentReference) "Ok" "KeepWorld" "KeepWorld" "KeepWorld" true)))

(fn DestroyAllMesh
  (bind _outactors (Actor|GetAttachedActors false))
  (while (> (Utilities|Array|Length _outactors) 0)
    (for _array_element _outactors
      (Actor|DestroyActor _array_element)))
  (Actor|DestroyActor))

(fn ChangeColorGreen
  (params (ColorValue :type Vector%204%20Structure))
  (bind (_x _y _z _w) (Math|Vector4|BreakVector4 ColorValue))
  (bind _returnvalue (Rendering|Material|CreateDynamicMaterialInstance (Variables|Default|GetVisibleMesh) 0 "/Game/Materials/BasicShapeMaterial.BasicShapeMaterial" "None" :!class /Script/Engine.PrimitiveComponent))
  (Rendering|Material|SetVectorParameterValue _returnvalue "Color" (Utilities|Struct|MakeLinearColor _x _y _z _w) :!class /Script/Engine.MaterialInstanceDynamic)
  (Rendering|Material|SetMaterial (Variables|Default|GetBase) 0 _returnvalue))